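; GM_WorldClock_Auto4 is a world clock test that advances a time counter and signals text updates.
; On BeginPlay, a looping one-second timer increments TimeToSet and passes the truncated value to CallUpdateText.
; A one-shot five-second timer prints an end-of-night debug message.
; Both timer handles are stored in TimeTest, so the second overwrites the first.
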(event `EnNight_Event`
  (`KismetSystemLibrary.PrintText` "End night"))

(event `self.ReceiveBeginPlay`
  (`|ExecutionSequence`
    (:`then_0`
      (bind _returnvalue (`KismetSystemLibrary.K2_SetTimerDelegate` (delegate `Update_Text`) 1.0 true))
      (set `self.time_test` _returnvalue))
    (:`then_1`
      (bind _returnvalue_2 (`KismetSystemLibrary.K2_SetTimerDelegate` (delegate `EnNight_Event`) 5.0))
      (set `self.time_test` _returnvalue_2))))

(event `Update_Text`
  (bind _result (`/Engine/EditorBlueprintResources/StandardMacros.IncrementFloat` (`self.TimeToSet`))
    (:`  `
      (`self.UpdateText` (`KismetMathLibrary.FTrunc` _result)))))

(fn `UserConstructionScript`)