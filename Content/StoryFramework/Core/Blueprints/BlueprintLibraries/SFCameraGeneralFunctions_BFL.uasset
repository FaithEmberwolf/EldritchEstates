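; Blueprint function library of StoryFramework camera helpers that act on player 0's camera manager.
; It attaches components to the camera, reads gamepad use and camera states, and clamps pitch, mostly through an SF camera manager message lookup.
; Field of view and distance setters branch on the current first or third person preset to send updated settings.
; Fades use either the native camera fade or a reused-or-created WidgetFade_W overlay.
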(fn `AttachComponentToSFCamera`
  (params (Target :type "SceneComponent Object Reference"))
  (locals (LensCameraManager :type "PlayerCameraManager Object Reference") (TargetComponent :type "SceneComponent Object Reference"))
  (bind _returnvalue (`GameplayStatics.GetPlayerCameraManager` null))
  (bind _output_get (set `local.TargetComponent` Target))
  (set `local.LensCameraManager` _returnvalue)
  (`SceneComponent.K2_AttachToComponent` _output_get (`PlayerCameraManager.TransformComponent` _returnvalue) "None" "KeepRelative" "SnapToTarget" "KeepRelative" true)
  (bind _sfcameramanagerref (message `/Game/StoryFramework/Core/Blueprints/BlueprintInterfaces/SFPlayerCameraManager_BPI.GetSFCameraManager` (`local.LensCameraManager`)))
  (`SceneComponent.K2_SetWorldRotation` (`local.TargetComponent`) (`PlayerCameraManager.GetCameraRotation` (`local.LensCameraManager`)) false false))

(fn `DetachComponentFromSFCamera`
  (params (Target :type "SceneComponent Object Reference"))
  (locals (TargetComponent :type "SceneComponent Object Reference"))
  (bind _output_get (set `local.TargetComponent` Target))
  (`SceneComponent.K2_DetachFromComponent` _output_get "KeepRelative" "KeepRelative" "KeepRelative" true))

(fn `FadeCamera`
  (params (FromAlpha :type "Float (single-precision)") (ToAlpha :type "Float (single-precision)") (Duration :type "Float (single-precision)") (Color :type "LinearColor Structure") (bShouldFadeAudio :type Boolean) (bHoldWhenFinished :type Boolean))
  (`PlayerCameraManager.StartCameraFade` (`GameplayStatics.GetPlayerCameraManager` null) FromAlpha ToAlpha Duration Color bShouldFadeAudio bHoldWhenFinished))

(fn `GetPlayRateLengthInSeconds`
  (params (`Length(InSec)` :type "Float (double-precision)"))
  (returns (`Length(Rate)` :type "Float (double-precision)"))
  (return (/ 1.0 `Length(InSec)`)))

(fn `GetSFCameraStates`
  (returns (CameraStates :type "/Game/StoryFramework/Core/Blueprints/Structures/SFCameraState_S Structure"))
  (bind _sfcameramanagerref (message `/Game/StoryFramework/Core/Blueprints/BlueprintInterfaces/SFPlayerCameraManager_BPI.GetSFCameraManager` (`GameplayStatics.GetPlayerCameraManager` null)))
  (return (`/Game/StoryFramework/Core/Blueprints/SFPlayerCamera_PCM.CameraStates` _sfcameramanagerref)))

(fn `IsUsingGamepad`
  (returns (`Return Value` :type Boolean))
  (bind _sfcameramanagerref (message `/Game/StoryFramework/Core/Blueprints/BlueprintInterfaces/SFPlayerCameraManager_BPI.GetSFCameraManager` (`GameplayStatics.GetPlayerCameraManager` null)))
  (return (`/Game/StoryFramework/Core/Blueprints/SFPlayerCamera_PCM.IsUsingGamepad` _sfcameramanagerref)))

(fn `SetCameraDistance`
  (params (CameraDistance :type "Float (double-precision)"))
  (locals (PlayerCameraManager :type "PlayerCameraManager Object Reference") (Distance :type "Float (double-precision)"))
  (bind _playercameramanager (`local.PlayerCameraManager`))
  (set `local.Distance` CameraDistance)
  (bind _output_get (set `local.PlayerCameraManager` (`GameplayStatics.GetPlayerCameraManager` null)))
  (bind _sfcameramanagerref (message `/Game/StoryFramework/Core/Blueprints/BlueprintInterfaces/SFPlayerCameraManager_BPI.GetSFCameraManager` _output_get))
  (switch `/Game/StoryFramework/Core/Blueprints/Enumerators/CameraPresets_E` (`/Game/StoryFramework/Core/Blueprints/SFPlayerCamera_PCM.CurrentCameraPreset` _sfcameramanagerref)
    (:`NewEnumerator3`
      (bind (_controllergeneralcamerasettings_sensitivitysettings _controllergeneralcamerasettings_initialcamerapreset _controllergeneralcamerasettings_generalcameralag _controllergeneralcamerasettings_thirdpersonsettings _controllergeneralcamerasettings_firstpersonsettings _controllergeneralcamerasettings_transitionsettings) (break `/Game/StoryFramework/Core/Blueprints/Structures/GeneralCameraSettings_S` (`/Game/StoryFramework/Core/Blueprints/SFPlayerCamera_PCM.ControllerGeneralCameraSettings` _sfcameramanagerref)))
      (message `/Game/StoryFramework/Core/Blueprints/BlueprintInterfaces/SFPlayerCameraManager_BPI.SetCameraSettings` _playercameramanager (make `/Game/StoryFramework/Core/Blueprints/Structures/GeneralCameraSettings_S` _controllergeneralcamerasettings_sensitivitysettings _controllergeneralcamerasettings_initialcamerapreset 15.0 (make `/Game/StoryFramework/Core/Blueprints/Structures/ThirdPersonSettings_S` (`local.Distance`)) _controllergeneralcamerasettings_firstpersonsettings _controllergeneralcamerasettings_transitionsettings (struct :`FieldOfView` 60.0 :`FixedTransform` (struct :`Rotation` (struct :`W` 1.0) :`Translation` (0.0 0.0 0.0) :`Scale3D` (1.0 1.0 1.0)) :`ControlRotation` (struct :`Yaw` 90.0) :`LockInputTransitioning` true))))
    (:`NewEnumerator4`
      (bind (_controllergeneralcamerasettings_sensitivitysettings_2 _controllergeneralcamerasettings_initialcamerapreset_2 _controllergeneralcamerasettings_generalcameralag_2 _controllergeneralcamerasettings_thirdpersonsettings_2 _controllergeneralcamerasettings_firstpersonsettings_2 _controllergeneralcamerasettings_transitionsettings_2) (break `/Game/StoryFramework/Core/Blueprints/Structures/GeneralCameraSettings_S` (`/Game/StoryFramework/Core/Blueprints/SFPlayerCamera_PCM.ControllerGeneralCameraSettings` _sfcameramanagerref)))
      (message `/Game/StoryFramework/Core/Blueprints/BlueprintInterfaces/SFPlayerCameraManager_BPI.SetCameraSettings` _playercameramanager (make `/Game/StoryFramework/Core/Blueprints/Structures/GeneralCameraSettings_S` _controllergeneralcamerasettings_sensitivitysettings_2 _controllergeneralcamerasettings_initialcamerapreset_2 15.0 _controllergeneralcamerasettings_thirdpersonsettings_2 (make `/Game/StoryFramework/Core/Blueprints/Structures/FirstPersonSettings_S` 80.0) _controllergeneralcamerasettings_transitionsettings_2 (struct :`FieldOfView` 60.0 :`FixedTransform` (struct :`Rotation` (struct :`W` 1.0) :`Translation` (0.0 0.0 0.0) :`Scale3D` (1.0 1.0 1.0)) :`ControlRotation` (struct :`Yaw` 90.0) :`LockInputTransitioning` true))))))

(fn `SetCameraFieldOfView`
  (params (FieldOfView :type "Float (double-precision)"))
  (locals (PlayerCameraManager :type "PlayerCameraManager Object Reference") (TargetFieldOfView :type "Float (double-precision)"))
  (bind _playercameramanager (`local.PlayerCameraManager`))
  (bind _targetfieldofview (`local.TargetFieldOfView`))
  (set `local.TargetFieldOfView` FieldOfView)
  (bind _output_get (set `local.PlayerCameraManager` (`GameplayStatics.GetPlayerCameraManager` null)))
  (bind _sfcameramanagerref (message `/Game/StoryFramework/Core/Blueprints/BlueprintInterfaces/SFPlayerCameraManager_BPI.GetSFCameraManager` _output_get))
  (switch `/Game/StoryFramework/Core/Blueprints/Enumerators/CameraPresets_E` (`/Game/StoryFramework/Core/Blueprints/SFPlayerCamera_PCM.CurrentCameraPreset` _sfcameramanagerref)
    (:`NewEnumerator3`
      (bind (_controllergeneralcamerasettings_sensitivitysettings _controllergeneralcamerasettings_initialcamerapreset _controllergeneralcamerasettings_generalcameralag _controllergeneralcamerasettings_thirdpersonsettings _controllergeneralcamerasettings_firstpersonsettings _controllergeneralcamerasettings_transitionsettings) (break `/Game/StoryFramework/Core/Blueprints/Structures/GeneralCameraSettings_S` (`/Game/StoryFramework/Core/Blueprints/SFPlayerCamera_PCM.ControllerGeneralCameraSettings` _sfcameramanagerref)))
      (message `/Game/StoryFramework/Core/Blueprints/BlueprintInterfaces/SFPlayerCameraManager_BPI.SetCameraSettings` _playercameramanager (make `/Game/StoryFramework/Core/Blueprints/Structures/GeneralCameraSettings_S` _controllergeneralcamerasettings_sensitivitysettings _controllergeneralcamerasettings_initialcamerapreset 15.0 (make `/Game/StoryFramework/Core/Blueprints/Structures/ThirdPersonSettings_S` 200.0 _targetfieldofview) _controllergeneralcamerasettings_firstpersonsettings _controllergeneralcamerasettings_transitionsettings (struct :`FieldOfView` 60.0 :`FixedTransform` (struct :`Rotation` (struct :`W` 1.0) :`Translation` (0.0 0.0 0.0) :`Scale3D` (1.0 1.0 1.0)) :`ControlRotation` (struct :`Yaw` 90.0) :`LockInputTransitioning` true))))
    (:`NewEnumerator4`
      (bind (_controllergeneralcamerasettings_sensitivitysettings_2 _controllergeneralcamerasettings_initialcamerapreset_2 _controllergeneralcamerasettings_generalcameralag_2 _controllergeneralcamerasettings_thirdpersonsettings_2 _controllergeneralcamerasettings_firstpersonsettings_2 _controllergeneralcamerasettings_transitionsettings_2) (break `/Game/StoryFramework/Core/Blueprints/Structures/GeneralCameraSettings_S` (`/Game/StoryFramework/Core/Blueprints/SFPlayerCamera_PCM.ControllerGeneralCameraSettings` _sfcameramanagerref)))
      (message `/Game/StoryFramework/Core/Blueprints/BlueprintInterfaces/SFPlayerCameraManager_BPI.SetCameraSettings` _playercameramanager (make `/Game/StoryFramework/Core/Blueprints/Structures/GeneralCameraSettings_S` _controllergeneralcamerasettings_sensitivitysettings_2 _controllergeneralcamerasettings_initialcamerapreset_2 15.0 _controllergeneralcamerasettings_thirdpersonsettings_2 (make `/Game/StoryFramework/Core/Blueprints/Structures/FirstPersonSettings_S` 80.0 _targetfieldofview) _controllergeneralcamerasettings_transitionsettings_2 (struct :`FieldOfView` 60.0 :`FixedTransform` (struct :`Rotation` (struct :`W` 1.0) :`Translation` (0.0 0.0 0.0) :`Scale3D` (1.0 1.0 1.0)) :`ControlRotation` (struct :`Yaw` 90.0) :`LockInputTransitioning` true))))))

(fn `SetCameraPitchClamps`
  (params (`View Pitch Min` :type "Float (single-precision)") (`View Pitch Max` :type "Float (single-precision)"))
  (bind _sfcameramanagerref (message `/Game/StoryFramework/Core/Blueprints/BlueprintInterfaces/SFPlayerCameraManager_BPI.GetSFCameraManager` (`GameplayStatics.GetPlayerCameraManager` null)))
  (`/Game/StoryFramework/Core/Blueprints/SFPlayerCamera_PCM.ClampCameraPitch` _sfcameramanagerref `View Pitch Min` `View Pitch Max`))

(fn `WidgetFadeCamera`
  (params (FadeDirection :type Integer) (`FadeSpeed (InSec)` :type "Float (double-precision)"))
  (locals (WidgetFadeRef :type "/Game/StoryFramework/Core/UserInterface/Widgets/WidgetFade_W Object Reference") (FadeDirRef :type Integer) (FadeSpeedRef :type "Float (double-precision)"))
  (bind _widgetfaderef (`local.WidgetFadeRef`))
  (set `local.FadeDirRef` FadeDirection)
  (set `local.FadeSpeedRef` `FadeSpeed (InSec)`)
  (bind _foundwidgets (`WidgetBlueprintLibrary.GetAllWidgetsOfClass` null "/Game/StoryFramework/Core/UserInterface/Widgets/WidgetFade_W.WidgetFade_W_C"))
  (bind _output (`|GetArrayItem` _foundwidgets))
  (`/Engine/EditorBlueprintResources/StandardMacros.IsValid` _output
    (:`Is Valid`
      (set `local.WidgetFadeRef` _output))
    (:`Is Not Valid`
      (bind _returnvalue (`|CreateWidget` "/Game/StoryFramework/Core/UserInterface/Widgets/WidgetFade_W.WidgetFade_W_C"))
      (set `local.WidgetFadeRef` _returnvalue)))
  (set `/Game/StoryFramework/Core/UserInterface/Widgets/WidgetFade_W.FadeDirection` (`local.FadeDirRef`) _widgetfaderef)
  (set `/Game/StoryFramework/Core/UserInterface/Widgets/WidgetFade_W.FadeSpeed(InSec)` (`local.FadeSpeedRef`) _widgetfaderef)
  (`/Game/StoryFramework/Core/UserInterface/Widgets/WidgetFade_W.StartFade` _widgetfaderef)
  (`UserWidget.AddToViewport` (`local.WidgetFadeRef`) 2))