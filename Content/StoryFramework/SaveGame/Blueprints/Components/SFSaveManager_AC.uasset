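; Story Framework save manager component that saves and loads game progress through one SFSaveGame_BP slot, with timed auto-save and a save popup.
; It stores player transform, view, camera settings, inventory, journal and dialog tags, substituting the previous camera preset during certain NPC dialog shots.
; It also stores spawned, destroyed and interacted actor records.
; Loading respawns actors, then matches level actors by object name to destroy them or restore their interaction state.
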(event `AutoSave (StoryFramework)`
  (params (`SaveIntervals(InSec)` :type "Float (double-precision)" :default 20.0))
  ;[0.04314 0.04314 0.05098] Systems (Root)
  (`KismetSystemLibrary.K2_SetTimer` null "AutoSaveLoop" `SaveIntervals(InSec)` true))

(event `AutoSaveLoop`
  ;[0.04314 0.04314 0.05098] Systems (Root)
  (`self.SaveGame (StoryFramework)`))

(event `SaveGame (StoryFramework)`
  (bind _interactionmanager (`/Game/StoryFramework/Core/Blueprints/BlueprintLibraries/SFGameplayFunctions_BFL.GetSFInteractionManager (Controller)`))
  (bind _assfgame_instance_bp (cast `/Game/StoryFramework/Core/SFGameInstance_BP` (`GameplayStatics.GetGameInstance`) :!pure true))
  ;[0.04314 0.04314 0.05098] Systems (Root)
  (bind _returnvalue (`GameplayStatics.CreateSaveGameObject` "/Game/StoryFramework/SaveGame/SFSaveGame_BP.SFSaveGame_BP_C"))
  (set `/Game/StoryFramework/SaveGame/SFSaveGame_BP.PlayerTransform` (`Actor.GetTransform` (`GameplayStatics.GetPlayerCharacter` 0)) _returnvalue) ; Save player location.
  (set `/Game/StoryFramework/SaveGame/SFSaveGame_BP.InventoryItems` (`/Game/StoryFramework/Core/Blueprints/Components/Core/SFInventoryManager_AC.InventoryItems` (`/Game/StoryFramework/Core/Blueprints/BlueprintLibraries/SFGameplayFunctions_BFL.GetSFInventoryManager (Controller)`)) _returnvalue) ; Save inventory.
  (bind _camerasettings (message `/Game/StoryFramework/Core/Blueprints/BlueprintInterfaces/SFPlayerCameraManager_BPI.GetSFCameraData` (`GameplayStatics.GetPlayerCameraManager` 0)))
  (bind _sfcameramanagerref (message `/Game/StoryFramework/Core/Blueprints/BlueprintInterfaces/SFPlayerCameraManager_BPI.GetSFCameraManager` (`GameplayStatics.GetPlayerCameraManager` 0)))
  (bind (_sensitivitysettings _initialcamerapreset _generalcameralag _thirdpersonsettings _firstpersonsettings _transitionsettings _fixedsettings) (break `/Game/StoryFramework/Core/Blueprints/Structures/GeneralCameraSettings_S` _camerasettings))
  (set `/Game/StoryFramework/SaveGame/SFSaveGame_BP.CameraSettings` (make `/Game/StoryFramework/Core/Blueprints/Structures/GeneralCameraSettings_S` _sensitivitysettings (select `bool` (and (`|EnumEquality` (`/Game/StoryFramework/Core/Blueprints/Components/Core/SFInteractionManager_AC.CurrentCameraPreset` _interactionmanager) "NewEnumerator7") (`/Game/StoryFramework/Core/Blueprints/Components/Core/SFInteractionManager_AC.IsInDialogWithNPC` _interactionmanager)) :`false` (`.InitialCameraPreset_21_BFA23052428F8F4269F26E9F944D9314` (break `/Game/StoryFramework/Core/Blueprints/Structures/GeneralCameraSettings_S` _camerasettings)) :`true` (`/Game/StoryFramework/Core/Blueprints/SFPlayerCamera_PCM.PreviousNonFixedCameraPreset` _sfcameramanagerref)) _generalcameralag _thirdpersonsettings _firstpersonsettings _transitionsettings _fixedsettings) _returnvalue) ; Save camera settings.
  (set `/Game/StoryFramework/SaveGame/SFSaveGame_BP.ControlRotation` (`Controller.GetControlRotation` (`GameplayStatics.GetPlayerController` 0)) _returnvalue) ; Save player rotation.
  (set `/Game/StoryFramework/SaveGame/SFSaveGame_BP.DestroyedActors` (`self.DestroyedActors`) _returnvalue) ; Save destroyed actors.
  (set `/Game/StoryFramework/SaveGame/SFSaveGame_BP.JournalEntries` (`/Game/StoryFramework/Core/Blueprints/Components/Core/SFInventoryManager_AC.JournalEntries` (`/Game/StoryFramework/Core/Blueprints/BlueprintLibraries/SFGameplayFunctions_BFL.GetSFInventoryManager (Controller)`)) _returnvalue) ; Save journal entries.
  (set `/Game/StoryFramework/SaveGame/SFSaveGame_BP.ConsequentialTags` (`/Game/StoryFramework/Core/Blueprints/Components/Core/SFInteractionManager_AC.ConsequentialTags` (`/Game/StoryFramework/Core/Blueprints/BlueprintLibraries/SFGameplayFunctions_BFL.GetSFInteractionManager (Controller)`)) _returnvalue) ; Save NPC dialog tags.
  (set `/Game/StoryFramework/SaveGame/SFSaveGame_BP.SpawnedActors` (`self.SpawnedActors`) _returnvalue) ; Save spawned actors.
  (set `/Game/StoryFramework/SaveGame/SFSaveGame_BP.InteractActors` (`self.InteractActors`) _returnvalue) ; Save interact actor info.
  (set `/Game/StoryFramework/SaveGame/SFSaveGame_BP.SystemData` (make `/Game/StoryFramework/SaveGame/Blueprints/Structures/SystemSaveData_S` (`KismetMathLibrary.Now`) (`/Game/StoryFramework/Core/SFGameInstance_BP.Sensitivity` _assfgame_instance_bp) (`/Game/StoryFramework/Core/SFGameInstance_BP.MasterVolume` _assfgame_instance_bp)) _returnvalue) ; Save system data info.
  (`GameplayStatics.SaveGameToSlot` _returnvalue "SFSaveSlot")
  (bind _returnvalue_2 (`|CreateWidget` "/Game/StoryFramework/Core/UserInterface/Widgets/PopupMaster_W.PopupMaster_W_C"))
  (`/Game/StoryFramework/Core/UserInterface/Widgets/PopupMaster_W.ShowSavePopup` _returnvalue_2)
  (`UserWidget.AddToViewport` _returnvalue_2 0))

(event `LoadGame (StoryFramework)`
  (bind _inventorymanager (`/Game/StoryFramework/Core/Blueprints/BlueprintLibraries/SFGameplayFunctions_BFL.GetSFInventoryManager (Controller)`))
  ;[0.04314 0.04314 0.05098] Systems (Root)
  (bind _returnvalue (`GameplayStatics.LoadGameFromSlot` "SFSaveSlot"))
  (bind _assfsave_game_bp (cast `/Game/StoryFramework/SaveGame/SFSaveGame_BP` _returnvalue))
  (`Actor.K2_SetActorTransform` (`GameplayStatics.GetPlayerCharacter` 0) (`/Game/StoryFramework/SaveGame/SFSaveGame_BP.PlayerTransform` _assfsave_game_bp) false false) ; Load player location.
  (message `/Game/StoryFramework/Core/Blueprints/BlueprintInterfaces/SFPlayerCameraManager_BPI.SetCameraSettings` (`GameplayStatics.GetPlayerCameraManager` 0) (`/Game/StoryFramework/SaveGame/SFSaveGame_BP.CameraSettings` _assfsave_game_bp)) ; Load camera settings.
  (`|ExecutionSequence`
    (:`then_0`
      (bind _inventoryitems (`/Game/StoryFramework/SaveGame/SFSaveGame_BP.InventoryItems` _assfsave_game_bp))
      (bind _keys (`BlueprintMapLibrary.Map_Keys` _inventoryitems))
      (`/Game/StoryFramework/Core/Blueprints/Components/Core/SFInventoryManager_AC.ClearInventory` _inventorymanager)
      (for _array_element _keys
        (`/Game/StoryFramework/Core/Blueprints/Components/Core/SFInventoryManager_AC.AddItemToInventory` _inventorymanager _array_element (`BlueprintMapLibrary.Map_Find` _inventoryitems _array_element) null)))
    (:`then_1`
      (`Controller.SetControlRotation` (`GameplayStatics.GetPlayerController` 0) (`/Game/StoryFramework/SaveGame/SFSaveGame_BP.ControlRotation` _assfsave_game_bp)) ; Load player rotation.
      (set `/Game/StoryFramework/Core/Blueprints/Components/Core/SFInventoryManager_AC.JournalEntries` (`/Game/StoryFramework/SaveGame/SFSaveGame_BP.JournalEntries` _assfsave_game_bp) (`/Game/StoryFramework/Core/Blueprints/BlueprintLibraries/SFGameplayFunctions_BFL.GetSFInventoryManager (Controller)`))
      (set `/Game/StoryFramework/Core/Blueprints/Components/Core/SFInteractionManager_AC.ConsequentialTags` (`/Game/StoryFramework/SaveGame/SFSaveGame_BP.ConsequentialTags` _assfsave_game_bp) (`/Game/StoryFramework/Core/Blueprints/BlueprintLibraries/SFGameplayFunctions_BFL.GetSFInteractionManager (Controller)`))
      (bind _output_get (set `self.SpawnedActors` (`/Game/StoryFramework/SaveGame/SFSaveGame_BP.SpawnedActors` _assfsave_game_bp)))
      (`|ExecutionSequence`
        (:`then_0`
          (if (`KismetArrayLibrary.Array_IsNotEmpty` _output_get)
            (for _array_element_2 _output_get
              (bind (_actorclass _actortransform _interactabledata _staticmeshactor) (break `/Game/StoryFramework/SaveGame/Blueprints/Structures/LevelActorSaveData_S` _array_element_2))
              (`/Engine/EditorBlueprintResources/StandardMacros.IsValid` _staticmeshactor
                (:`Is Valid`
                  (bind _returnvalue_2 (`|SpawnActorFromClass` "/Script/Engine.StaticMeshActor" _actortransform "Undefined" "MultiplyWithRoot" null null))
                  (bind _staticmeshcomponent (`StaticMeshActor.StaticMeshComponent` _returnvalue_2))
                  (`SceneComponent.SetMobility` _staticmeshcomponent "Movable")
                  (`StaticMeshComponent.SetStaticMesh` _staticmeshcomponent _staticmeshactor))
                (:`Is Not Valid`
                  (bind _returnvalue_3 (`|SpawnActorFromClass` _actorclass _actortransform "Undefined" "SelectDefaultAtRuntime" null null))
                  (bind _asinteractable_base_bp (cast `/Game/StoryFramework/Core/Blueprints/InteractableBase_BP` _returnvalue_3))
                  (set `/Game/StoryFramework/Core/Blueprints/InteractableBase_BP.InteractionData` _interactabledata _asinteractable_base_bp)
                  (`/Game/StoryFramework/Core/Blueprints/InteractableBase_BP.UpdateCosmetics` _asinteractable_base_bp))))))
        (:`then_1`
          (bind _output_get_2 (set `self.DestroyedActors` (`/Game/StoryFramework/SaveGame/SFSaveGame_BP.DestroyedActors` _assfsave_game_bp)))
          (`|ExecutionSequence`
            (:`then_0`
              (bind _outactors (`GameplayStatics.GetAllActorsOfClass` "/Script/Engine.Actor"))
              (for _array_element_3 _outactors
                (bind _returnvalue_4 (`KismetSystemLibrary.GetObjectName` _array_element_3))
                (bind _returnvalue_5 (`KismetArrayLibrary.Array_Find` _output_get_2 _returnvalue_4))
                (if (and (`KismetArrayLibrary.Array_Contains` _output_get_2 _returnvalue_4) (> _returnvalue_5 -1))
                  (if (`KismetStringLibrary.EqualEqual_StrStr` _returnvalue_4 (`|GetArrayItem` (`self.DestroyedActors`) _returnvalue_5))
                    (`Actor.K2_DestroyActor` _array_element_3)))))
            (:`then_1`
              (bind _output_get_3 (set `self.InteractActors` (`/Game/StoryFramework/SaveGame/SFSaveGame_BP.InteractActors` _assfsave_game_bp)))
              (`|ExecutionSequence`
                (:`then_0`
                  (bind _outactors_2 (`GameplayStatics.GetAllActorsOfClass` "/Script/Engine.Actor"))
                  (for _array_element_4 _outactors_2
                    (bind (_value _returnvalue_6) (`BlueprintMapLibrary.Map_Find` _output_get_3 (`KismetSystemLibrary.GetObjectName` _array_element_4)))
                    (if _returnvalue_6
                      (bind _asinteractable_base_bp_2 (cast `/Game/StoryFramework/Core/Blueprints/InteractableBase_BP` _array_element_4))
                      (`/Game/StoryFramework/Core/Blueprints/InteractableBase_BP.LoadFromDataString` _asinteractable_base_bp_2 _value))))
                (:`then_1`)))))))))