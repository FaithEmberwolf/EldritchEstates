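; BP_Testing is a test Blueprint in FailedTests that mixes debug exercises with a prototype farming plot.
; BeginPlay prints coloured text, draws a debug sphere and spawns a fire emitter that it shifts twice on delays.
; HandlePlotInteraction plants a fixed-type seedling in an empty plot.
; ProgressPlantStage advances watered growth stages, but switches on literal Seedling rather than PlantStage, so it only ever reaches the first growing stage.
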(event `self.ReceiveBeginPlay`
  (bind _center (`self.Center`))
  (`KismetSystemLibrary.PrintString` "Hello" true true (`self.HelloTextColour`) 10.0)
  (`KismetSystemLibrary.PrintString` "World" true true (`self.WorldTextColour`) 10.0)
  (`KismetSystemLibrary.DrawDebugSphere` _center 100.0 12 (struct :`A` 1.0) 10.0 1.0)
  (bind _returnvalue (`GameplayStatics.SpawnEmitterAtLocation` "/Game/StarterContent/Particles/P_Fire.P_Fire" _center))
  (`KismetSystemLibrary.Delay` 2.0)
  (`SceneComponent.K2_AddWorldOffset` _returnvalue (0.0 200.0 0.0) false false)
  (`KismetSystemLibrary.Delay` 2.0)
  (`SceneComponent.K2_AddWorldOffset` _returnvalue (0.0 200.0 0.0) false false))

(event `Handle Plot Interaction`
  ;[1 1 1] Handle Player Interaction
  (if (`self.BIsEmpty`)
    (if (`self.Player Interacted`)
      ;;[1 1 1] Needs to take result of whats in players hand
      (set `self.PlantType` "NewEnumerator1")
      (set `self.PlantStage` "NewEnumerator0")
      (set `self.BIsEmpty` false)
      (set `self.Player Interacted` false))))

(event `Progress Plant Stage`
  (bind _biswatered (`self.BIsWatered`))
  ;[1 1 1] Stage Manager
  (switch `/Game/Johns_Content/Variables/Enums/E_PlantState` "NewEnumerator0"
    (:`NewEnumerator0`
      ;;[1 1 1] The conditions need to be if it is water and "x" amount of time has passed while watered (The x condition requires the world clock)
      (if _biswatered
        (set `self.PlantStage` "NewEnumerator1")
        (set `self.BIsWatered` false :!label _label)))
    (:`NewEnumerator1`
      (if _biswatered
        (set `self.PlantStage` "NewEnumerator2")
        (goto _label)))
    (:`NewEnumerator2`
      (if _biswatered
        (set `self.PlantStage` "NewEnumerator3")
        (goto _label)))))

(fn `UserConstructionScript`)