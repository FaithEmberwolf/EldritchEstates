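; Base crop interactable for farm plots, built on Story Framework interaction, that shows a plant's growth state and becomes harvestable.
; A looping 0.1-second timer polls State and Type without advancing them, setting the mesh from DT_Plants.
; At one specific state it sends pumpkin or parsnip name, harvest and pickup data to the interaction manager.
; Construction and interaction-data updates refresh the mesh and collision sphere radius.
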(event `self.InteractWith`
  (params (DataString :type String)))

(event `self.UpdateInteractionData`
  (params (InteractionData :type "/Game/StoryFramework/Core/Blueprints/Structures/InteractableData_S Structure"))
  (set `self.InteractionData` InteractionData)
  (`/Game/StoryFramework/Core/Blueprints/Components/Other/SFInteractionWidget_SC.UpdateInitialization` (`self.SFInteractionWidget_SC`))
  (`self.UpdateCosmetics`)
  (`SphereComponent.SetSphereRadius` (`self.Sphere`) (`self.CustomCollisionRadius`) true))

(event `UpdateCosmetics`
  (`StaticMeshComponent.SetStaticMesh` (`self.StaticMesh`) (`.ObjectMesh_44_EE9024FA467AC4603952289EAC52AD36` (break `/Game/StoryFramework/Core/Blueprints/Structures/InteractableData_S` (`self.InteractionData`))))
  (`/Game/StoryFramework/Core/Blueprints/Components/Other/SFInteractionWidget_SC.UpdateInitialization` (`self.SFInteractionWidget_SC`)))

(event `LoadFromDataString`
  (params (DataString :type String)))

(event `self.ReceiveBeginPlay`
  (`KismetSystemLibrary.K2_SetTimerDelegate` (delegate `Incriment State`) 0.1 true))

(event `Incriment State`
  (bind _state (`self.State`))
  (bind _type (`self.Type`))
  (if (`|EnumInequality` _state "NewEnumerator4")
    (if (`|EnumInequality` _type "NewEnumerator3")
      (bind _staticmesh (`self.ChangeTheStaticMesh` _state _type))
      (if (`|EnumEquality` _state "NewEnumerator3")
        (if (`|EnumEquality` _type "NewEnumerator1")
          (`/Game/StoryFramework/Core/Blueprints/Components/Core/SFInteractionManager_AC.UpdateActorInteractionData` (`/Game/StoryFramework/Core/Blueprints/BlueprintLibraries/SFGameplayFunctions_BFL.GetSFInteractionManager (Controller)`) self (make `/Game/StoryFramework/Core/Blueprints/Structures/InteractableData_S` (`self.Pumpkin Name`) _staticmesh (`self.Interaction Data Interaction Prompt Offset`) (`self.Interaction Data Display Prompt From Range`) (`self.Pumpkin harvesting`) (`self.Pickup Method for Pumpkin`) (struct) (struct)))
          (else
            (`/Game/StoryFramework/Core/Blueprints/Components/Core/SFInteractionManager_AC.UpdateActorInteractionData` (`/Game/StoryFramework/Core/Blueprints/BlueprintLibraries/SFGameplayFunctions_BFL.GetSFInteractionManager (Controller)`) self (make `/Game/StoryFramework/Core/Blueprints/Structures/InteractableData_S` (`self.Parsnip Name`) _staticmesh (`self.Interaction Data Interaction Prompt Offset`) (`self.Interaction Data Display Prompt From Range`) (`self.Parsnip harvesting`) (`self.Pickup Method For Parsnip`) (struct) (struct)))))))))

(fn `ChangeTheStaticMesh`
  (params (State :type "/Game/Johns_Content/Variables/Enums/E_PlantState Enum" :default "NewEnumerator4") (`Plant Type` :type "/Game/Johns_Content/Variables/Enums/E_PlantType Enum" :default "NewEnumerator1"))
  (returns (StaticMesh :type "StaticMesh Object Reference"))
  (bind _returnvalue (`|GetDataTableRow` "/Game/Johns_Content/Variables/DataTables/DT_Plants.DT_Plants" (`KismetStringLibrary.Conv_StringToName` (`|GetEnumeratorNameAsString` `Plant Type`)))
    (:`then`
      (bind _value (`BlueprintMapLibrary.Map_Find` (`.PlantMesh_19_D2298918410AAD5E809B5B99A4719ABE` (break `/Game/Johns_Content/Structs/S_PlantBase` _returnvalue)) State))
      (`StaticMeshComponent.SetStaticMesh` (`self.StaticMesh`) _value)
      (return _value))
    (:`RowNotFound`
      (`KismetSystemLibrary.PrintString` "\"Get Data Table Row DT_Plants\" Row Not Found" true true (struct :`G` 0.66 :`B` 1.0 :`A` 1.0) 50.0 "Datatable Error"))))

(fn `GetInteractionData`
  (returns (InteractionData :type "/Game/StoryFramework/Core/Blueprints/Structures/InteractableData_S Structure"))
  (return (`self.InteractionData`)))

(fn `UserConstructionScript`
  (`self.UpdateCosmetics`)
  (`SphereComponent.SetSphereRadius` (`self.Sphere`) (`self.CustomCollisionRadius`) true))