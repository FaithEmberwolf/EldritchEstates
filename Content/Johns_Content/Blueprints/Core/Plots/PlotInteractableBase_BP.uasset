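; Base interactable farm plot that tracks a crop's type, growth state and watering, with functions for planting and harvesting.
; A looping timer advances growth while watered and planted, pulling each stage's crop mesh from DT_Plants by type and state.
; Tick swaps the dirt between wet and dry materials, and harvesting resets the plot and returns the plant type.
; Tilled visibility, inventory checks and state-based interaction updates are unfinished or not wired in.
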(event `self.ReceiveTick`
  (params (DeltaSeconds :type "Float (single-precision)"))
  (`self.SwapMaterialIfWatered`)
  (bind _output_get (set `self.CurrentDuration` (+ DeltaSeconds (`self.CurrentDuration`))))
  (if (> _output_get (`self.ThreshholdTime`))
    (set `self.CurrentDuration` 0.0)))

(event `self.ReceiveBeginPlay`
  (`KismetSystemLibrary.K2_SetTimerDelegate` (delegate `Incriment State`) 5.0 true))

(event `Incriment State`
  (if (`self.Watered?`)
    (if (`|EnumInequality` (`self.Type`) "NewEnumerator3")
      (bind _output_get (`self.ChangeState`))
      (`KismetSystemLibrary.PrintString` (`|GetEnumeratorNameAsString` _output_get))
      (else
        (`KismetSystemLibrary.PrintString` "Type is Null" true true (struct :`R` 1.0 :`G` 0.039766 :`A` 1.0) 2.0 "Type Response")))))

(fn `ChangeState`
  (returns (Output_Get :type "/Game/Johns_Content/Variables/Enums/E_PlantState Enum"))
  (bind _returnvalue (`KismetMathLibrary.Conv_ByteToInt` (`self.State`)))
  (if (not (>= _returnvalue 4))
    (bind _result (`/Engine/EditorBlueprintResources/StandardMacros.IncrementInt` _returnvalue)
      (:`  `
        (bind _output_get (set `self.State` (cast `/Game/Johns_Content/Variables/Enums/E_PlantState` (`KismetMathLibrary.Conv_IntToByte` _result))))
        (`self.ChangeTheStaticMesh` _output_get (`self.Type`))
        (`KismetSystemLibrary.PrintString` (`|GetEnumeratorNameAsString` _output_get) true true (struct :`G` 0.66 :`B` 1.0 :`A` 1.0) 10.0 "Current State")
        (return _output_get)))))

(fn `ChangeTheStaticMesh`
  (params (State :type "/Game/Johns_Content/Variables/Enums/E_PlantState Enum" :default "NewEnumerator4") (`Plant Type` :type "/Game/Johns_Content/Variables/Enums/E_PlantType Enum" :default "NewEnumerator1"))
  (bind _returnvalue (`|GetDataTableRow` "/Game/Johns_Content/Variables/DataTables/DT_Plants.DT_Plants" (`KismetStringLibrary.Conv_StringToName` (`|GetEnumeratorNameAsString` `Plant Type`)))
    (:`then`
      (`StaticMeshComponent.SetStaticMesh` (`self.Crop`) (`BlueprintMapLibrary.Map_Find` (`.PlantMesh_19_D2298918410AAD5E809B5B99A4719ABE` (break `/Game/Johns_Content/Structs/S_PlantBase` _returnvalue)) State)))
    (:`RowNotFound`
      (`KismetSystemLibrary.PrintString` "\"Get Data Table Row DT_Plants\" Row Not Found" true true (struct :`G` 0.66 :`B` 1.0 :`A` 1.0) 50.0 "Datatable Error"))))

(fn `CheckIfPlotStateIsNull`
  (if (`|EnumEquality` (`self.State`) "NewEnumerator4")
    _))

(fn `Harvesting`
  (returns (`Crop Harvested` :type "/Game/Johns_Content/Variables/Enums/E_PlantType Enum"))
  (locals (`Local Type` :type "/Game/Johns_Content/Variables/Enums/E_PlantType Enum"))
  (set `self.State` "NewEnumerator4")
  (bind _output_get (set `local.Local Type` (`self.Type`)))
  (set `self.Type` "NewEnumerator3")
  (`self.ChangeTheStaticMesh` (`self.State`) (`self.Type`))
  (set `self.Watered?` false)
  (return _output_get))

(fn `Planting`
  (params (`Plant Type` :type "/Game/Johns_Content/Variables/Enums/E_PlantType Enum" :default "NewEnumerator1") (`Plant State` :type "/Game/Johns_Content/Variables/Enums/E_PlantState Enum" :default "NewEnumerator4"))
  (returns (State :type "/Game/Johns_Content/Variables/Enums/E_PlantState Enum") (Type :type "/Game/Johns_Content/Variables/Enums/E_PlantType Enum"))
  (bind _output_get (set `self.Type` `Plant Type`))
  (bind _output_get_2 (set `self.State` `Plant State`))
  (return _output_get_2 _output_get))

(fn `ReturnPlotState`
  (returns (`Plant State` :type "/Game/Johns_Content/Variables/Enums/E_PlantState Enum"))
  (return (`self.State`)))

(fn `ShowPlotIfTilled`
  (if (`self.Tilled?`)
    (`SceneComponent.SetVisibility` (`self.StaticMesh`) true false)
    (else
      (`SceneComponent.SetVisibility` (`self.StaticMesh`) false false))))

(fn `SwapMaterialIfWatered`
  (if (`self.Watered?`)
    (`PrimitiveComponent.SetMaterial` (`self.StaticMesh`) 0 "/Game/Johns_Content/Materials/Dirt/M_DirtPatch_Wet.M_DirtPatch_Wet")
    (else
      (`PrimitiveComponent.SetMaterial` (`self.StaticMesh`) 0 "/Game/Johns_Content/Materials/Dirt/M_DirtPatch.M_DirtPatch"))))

(fn `UserConstructionScript`
  (`parent.UserConstructionScript`))