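; Replicated farm plot actor that grows a planted seed while it has water, controlled through interface events to plant, water and reset.
; On the server, looping timers advance growth and drain water, pausing when dry and clearing at maturity.
; Setters write to a shared PlantState struct, whose OnRep toggles mesh visibility, resumes paused growth and drives a timeline that scales the mesh.
; A separate OnRep applies the plant's mesh and starting scale.
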(event `/Game/FarmingSystem/Blueprints/Interfaces/BPI_FarmingSystem.BPI_ResetFarmActor`
  ;[1 1 1] INTERFACE EVENTS
  (`/Engine/EditorBlueprintResources/ActorMacros.Switch Has Authority`
    (:`Authority`
      (`self.SetFinishedGrowing` false)
      (`self.SetGrowthPercent` 0.0)
      (`self.SetSeedPlanted` false))))

(event `/Game/FarmingSystem/Blueprints/Interfaces/BPI_FarmingSystem.BPI_SetPlantData`
  (params (Data :type "/Game/FarmingSystem/Blueprints/Data/Structs/STR_FarmingSystem Structure"))
  ;[1 1 1] INTERFACE EVENTS
  (`/Engine/EditorBlueprintResources/ActorMacros.Switch Has Authority`
    (:`Authority`
      (`self.SetPlantData` Data)
      (`self.SetSeedPlanted` true)
      (bind _returnvalue (`KismetSystemLibrary.K2_SetTimerDelegate` (`|CreateDelegate` :!event `PlantGrowth`) 1.0 true))
      (set `self.PlantGrowthTimer` _returnvalue)
      (`self.StartDrainingWater`))))

(event `/Game/FarmingSystem/Blueprints/Interfaces/BPI_FarmingSystem.BPI_AddWater`
  (params (Amount :type "Float (double-precision)"))
  ;[1 1 1] INTERFACE EVENTS
  (`/Engine/EditorBlueprintResources/ActorMacros.Switch Has Authority`
    (:`Authority`
      (`self.SetWaterAmount` (+ Amount (`self.GetWaterAmount`))))))

(event `StartDrainingWater`
  ;[1 1 1] START DRAINING WATER
  (`/Engine/EditorBlueprintResources/ActorMacros.Switch Has Authority`
    (:`Authority`
      (bind _returnvalue (`KismetSystemLibrary.K2_SetTimerDelegate` (`|CreateDelegate` :!event `ReduceWater`) (`.WaterDrainRate_37_46013C6E4106D0AB5530D0B439F7C7A1` (break `/Game/FarmingSystem/Blueprints/Data/Structs/STR_FarmingSystem` (`self.PlantData`))) true))
      (set `self.WaterDrainTimer` _returnvalue))))

(event `GrowPlantMesh`
  ;[1 1 1] PLANT GROW TIMELINE
  (bind (_direction _growthalpha) (`Timeline|GrowthTimeLine` :!via `PlayFromStart`)
    (:`Update`
      (`SceneComponent.SetWorldScale3D` (`self.PlantMesh`) (`KismetMathLibrary.VLerp` (`SceneComponent.K2_GetComponentScale` (`self.PlantMesh`)) (`KismetMathLibrary.Conv_DoubleToVector` (* (`.PlantMatureScale_21_6A7B8C774369A5465E1718B8878E227C` (break `/Game/FarmingSystem/Blueprints/Data/Structs/STR_FarmingSystem` (`self.PlantData`))) (`self.GetGrowthPercent`))) _growthalpha)))))

(fn `BPI_GetFarmActorMesh`
  (returns (Mesh :type "StaticMeshComponent Object Reference"))
  (return (`self.Soil`)))

(fn `BPI_GetPlantData`
  (returns (PlantData :type "/Game/FarmingSystem/Blueprints/Data/Structs/STR_FarmingSystem Structure") (PlantState :type "/Game/FarmingSystem/Blueprints/Data/Structs/STR_PlantState Structure"))
  (return (`self.PlantData`) (`self.PlantState`)))

(fn `GetFinishedGrowing`
  (returns (FinishedGrowing :type Boolean))
  (return (`.FinishedGrowing_3_2F31DF0645566BA76D38C98D3ACAB7A4` (break `/Game/FarmingSystem/Blueprints/Data/Structs/STR_PlantState` (`self.PlantState`)))))

(fn `GetGrowthPercent`
  (returns (GrowthPercent :type "Float (double-precision)"))
  (return (`.GrowthPercent_8_1742713942EEC2D2AB0CEABDAEB62C9D` (break `/Game/FarmingSystem/Blueprints/Data/Structs/STR_PlantState` (`self.PlantState`)))))

(fn `GetHasWater`
  (returns (ReturnValue :type Boolean))
  (return (> (`.CurrentWaterAmount_10_079907774EDF4B4A7342EB8053F626EA` (break `/Game/FarmingSystem/Blueprints/Data/Structs/STR_PlantState` (`self.PlantState`))) 0.0)))

(fn `GetSeedPlanted`
  (returns (SeedPlanted :type Boolean))
  (return (`.SeedPlanted_1_15E3D9AB4465F80843FB5D9848F33BE6` (break `/Game/FarmingSystem/Blueprints/Data/Structs/STR_PlantState` (`self.PlantState`)))))

(fn `GetWaterAmount`
  (returns (CurrentWaterAmount :type "Float (double-precision)"))
  (return (`.CurrentWaterAmount_10_079907774EDF4B4A7342EB8053F626EA` (break `/Game/FarmingSystem/Blueprints/Data/Structs/STR_PlantState` (`self.PlantState`)))))

(fn `OnRep_FarmData`
  (`StaticMeshComponent.SetStaticMesh` (`self.PlantMesh`) (`.PlantMesh_25_69838FF64A6C27D3FDC1CFA82B7F7157` (break `/Game/FarmingSystem/Blueprints/Data/Structs/STR_FarmingSystem` (`self.PlantData`))))
  (`SceneComponent.SetWorldScale3D` (`self.PlantMesh`) (`KismetMathLibrary.Conv_DoubleToVector` (`.PlantBeginScale_19_3547C4794EEC7BC2B55147BF4D7B99C1` (break `/Game/FarmingSystem/Blueprints/Data/Structs/STR_FarmingSystem` (`self.PlantData`)))))
  (return))

(fn `OnRep_PlantState`
  (`SceneComponent.SetVisibility` (`self.PlantMesh`) (`self.GetSeedPlanted`) false)
  (if (`KismetSystemLibrary.K2_IsTimerPausedHandle` (`self.PlantGrowthTimer`))
    (if (> (`self.GetWaterAmount`) 0.0)
      (`KismetSystemLibrary.K2_UnPauseTimerHandle` (`self.PlantGrowthTimer`))
      (return))
    (elif (`self.GetFinishedGrowing`)
      (`SceneComponent.SetWorldScale3D` (`self.PlantMesh`) (`KismetMathLibrary.Conv_DoubleToVector` (`.PlantMatureScale_21_6A7B8C774369A5465E1718B8878E227C` (break `/Game/FarmingSystem/Blueprints/Data/Structs/STR_FarmingSystem` (`self.PlantData`)))))
      (return)
      (else
        (`TimelineComponent.SetPlayRate` (`self.GrowthTimeLine`) (/ 1.0 (`.GrowthTime_5_07B9DD8B43BBEC038BD14497AFE1A1B4` (break `/Game/FarmingSystem/Blueprints/Data/Structs/STR_FarmingSystem` (`self.PlantData`)))))
        (`self.GrowPlantMesh`)
        (return)))))

(fn `PlantGrowth`
  (`/Engine/EditorBlueprintResources/ActorMacros.Switch Has Authority`
    (:`Authority`
      (if (`self.GetHasWater`)
        (`self.SetGrowthPercent` (+ (`self.GetGrowthPercent`) (/ 1.0 (`.GrowthTime_5_07B9DD8B43BBEC038BD14497AFE1A1B4` (break `/Game/FarmingSystem/Blueprints/Data/Structs/STR_FarmingSystem` (`self.PlantData`))))))
        (if (>= (`self.GetGrowthPercent`) 1.0)
          (`self.SetFinishedGrowing` true)
          (return)
          (else
            (return)))
        (else
          (`KismetSystemLibrary.K2_PauseTimerHandle` (`self.PlantGrowthTimer`))
          (return))))
    (:`Remote`
      (return))))

(fn `ReduceWater`
  (`/Engine/EditorBlueprintResources/ActorMacros.Switch Has Authority`
    (:`Authority`
      (`self.SetWaterAmount` (`KismetMathLibrary.FClamp` (- (`self.GetWaterAmount`) (`.WaterDrainAmount_34_531397214252805318BBA4A46DA248F3` (break `/Game/FarmingSystem/Blueprints/Data/Structs/STR_FarmingSystem` (`self.PlantData`)))) 0.0 100.0)))))

(fn `SetFinishedGrowing`
  (params (FinishedGrowing :type Boolean))
  (locals (LocalFinishedGrowing :type Boolean))
  (set `local.LocalFinishedGrowing` FinishedGrowing)
  (`/Engine/EditorBlueprintResources/ActorMacros.Switch Has Authority`
    (:`Authority`
      (bind _structout (setmembers `/Game/FarmingSystem/Blueprints/Data/Structs/STR_PlantState` :`StructRef` (`self.PlantState`) :`FinishedGrowing` (`local.LocalFinishedGrowing`)))
      (set `self.PlantState` _structout)
      (if (`local.LocalFinishedGrowing`)
        (`KismetSystemLibrary.K2_ClearAndInvalidateTimerHandle` (`self.PlantGrowthTimer`))
        (`KismetSystemLibrary.K2_ClearAndInvalidateTimerHandle` (`self.WaterDrainTimer`))
        (return)
        (else
          (return))))
    (:`Remote`
      (return))))

(fn `SetGrowthPercent`
  (params (GrowthPercent :type "Float (double-precision)"))
  (`/Engine/EditorBlueprintResources/ActorMacros.Switch Has Authority`
    (:`Authority`
      (bind _structout (setmembers `/Game/FarmingSystem/Blueprints/Data/Structs/STR_PlantState` :`StructRef` (`self.PlantState`) :`GrowthPercent` GrowthPercent))
      (set `self.PlantState` _structout)
      (return))
    (:`Remote`
      (return))))

(fn `SetPlantData`
  (params (PlantData :type "/Game/FarmingSystem/Blueprints/Data/Structs/STR_FarmingSystem Structure"))
  (`/Engine/EditorBlueprintResources/ActorMacros.Switch Has Authority`
    (:`Authority`
      (set `self.PlantData` PlantData)
      (return))))

(fn `SetSeedPlanted`
  (params (SeedPlanted :type Boolean))
  (`/Engine/EditorBlueprintResources/ActorMacros.Switch Has Authority`
    (:`Authority`
      (bind _structout (setmembers `/Game/FarmingSystem/Blueprints/Data/Structs/STR_PlantState` :`StructRef` (`self.PlantState`) :`SeedPlanted` SeedPlanted))
      (set `self.PlantState` _structout)
      (return))
    (:`Remote`
      (return))))

(fn `SetWaterAmount`
  (params (CurrentWaterAmount :type "Float (double-precision)"))
  (`/Engine/EditorBlueprintResources/ActorMacros.Switch Has Authority`
    (:`Authority`
      (bind _structout (setmembers `/Game/FarmingSystem/Blueprints/Data/Structs/STR_PlantState` :`StructRef` (`self.PlantState`) :`CurrentWaterAmount` (`KismetMathLibrary.FClamp` CurrentWaterAmount 0.0 100.0)))
      (set `self.PlantState` _structout)
      (if (`self.GetHasWater`)
        (if (`KismetSystemLibrary.K2_IsTimerPausedHandle` (`self.WaterDrainTimer`))
          (`KismetSystemLibrary.K2_UnPauseTimerHandle` (`self.WaterDrainTimer`)))
        (else
          (`KismetSystemLibrary.K2_PauseTimerHandle` (`self.WaterDrainTimer`))))
      (return))
    (:`Remote`
      (return))))

(fn `UserConstructionScript`)