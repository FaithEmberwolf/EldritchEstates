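; Replicated farming component for a player pawn or controller that handles placing farm plots, planting, watering and harvesting.
; Placement spawns a farm actor that follows camera box traces, optionally snapping beside existing plots and checking overlap, with its transform sent to the server and applied through OnRep.
; Plant actions go through BPI_FarmingSystem, with distance checks on watering and harvesting; harvest reward logic is a stub.
; Client events drive the HUD interaction prompt, seed selection widget and feedback messages.
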(event `self.ReceiveBeginPlay`
  ;[1 1 1] BEGIN PLAY / INIT
  (bind _output_get (set `self.OwningActor` (`self.GetOwner`)))
  (`/Engine/EditorBlueprintResources/StandardMacros.IsValid` _output_get :!label _label
    (:`Is Valid`
      (`self.SetIsReplicated` true)
      (`self.IsLocal`
        (:`True`
          (bind _returnvalue (`|CreateWidget` "/Game/FarmingSystem/Blueprints/Widgets/WBP_HUD.WBP_HUD_C"))
          (bind _output_get_2 (set `self.HUD` _returnvalue))
          (`UserWidget.AddToViewport` _output_get_2 0))
        (:`false`
          _))
      (if (`self.bEnableTraceInteraction`)
        (`KismetSystemLibrary.Delay` 2.0) ; Wait for the HUD to initialize.
        (`KismetSystemLibrary.K2_SetTimerDelegate` (`|CreateDelegate` :!event `CL_FindInteractableObjects`) 0.1 true)))
    (:`Is Not Valid`
      (`KismetSystemLibrary.Delay` 0.2)
      (goto _label))))

(event `SRV_PlantSeed`
  (params (FarmActor :type "Actor Object Reference") (PlantData :type "/Game/FarmingSystem/Blueprints/Data/Structs/STR_FarmingSystem Structure"))
  ;[1 0.02544 0.1955] SERVER EVENTS
  ;;[1 1 1] PLANT SEED
  (`self.PlantSeed` FarmActor PlantData))

(event `CL_FindInteractableObjects`
  ;[0.2546 1 0.2921] CLIENT EVENTS
  ;;[1 1 1] FIND INTERACTABLE OBJECTS
  (`self.FindInteractableObjects`))

(event `SRV_SetFarmingState`
  ;[1 0.02544 0.1955] SERVER EVENTS
  ;;[1 1 1] SET FARMING STATE
  (`self.SetFarmingState` (not (`self.bPlacementState`))))

(event `CL_UpdateFarmActorPlacementLocation`
  ;[0.2546 1 0.2921] CLIENT EVENTS
  ;;[1 1 1] UPDATE FARM ACTOR PLACEMENT
  (`self.UpdateFarmActorPlacementLocation`))

(event `CL_SetFarmActorRotation`
  (params (Amount :type "Float (double-precision)"))
  ;[0.2546 1 0.2921] CLIENT EVENTS
  ;;[1 1 1] ADD ROTATION TO FARM ACTOR
  (set `self.FarmActorRotation` (`KismetMathLibrary.MakeRotator` 0.0 0.0 (+ (.yaw (`self.FarmActorRotation`)) Amount))))

(event `SRV_FinalizePlacement`
  ;[1 0.02544 0.1955] SERVER EVENTS
  ;;[1 1 1] FINALIZE PLACEMENT OF FARM ACTOR
  (`self.FinalizePlacement`))

(event `SRV_UpdateFarmActorLocation`
  (params (NewTransform :type "Transform Structure"))
  ;[1 0.02544 0.1955] SERVER EVENTS
  ;;[1 1 1] UPDATE FARM ACTOR LOCATION
  (set `self.FarmActorTransform` NewTransform))

(event `CL_CreatePlantsSelectionWidget`
  (params (FarmActor :type "Actor Object Reference"))
  ;[0.2546 1 0.2921] CLIENT EVENTS
  ;;[1 1 1] CREATE PLANT SELECTION WIDGET
  (`self.CreatePlantSelectionWidget` FarmActor))

(event `SRV_SpawnFarmActor`
  ;[1 0.02544 0.1955] SERVER EVENTS
  ;;[1 1 1] SPAWN FARM ACTOR
  (`self.SpawnFarmActor`))

(event `CL_InteractWithFarmActor`
  ;[0.2546 1 0.2921] CLIENT EVENTS
  ;;[1 1 1] INTERACT WITH FARM ACTOR
  (bind _asbp_farm_actor (cast `/Game/FarmingSystem/Blueprints/BP_FarmActor` (`.HitActor` (`GameplayStatics.BreakHitResult` (`self.FindCameraViewPoint`)))))
  (`self.CL_CreatePlantsSelectionWidget` _asbp_farm_actor))

(event `SRV_AddWater`
  (params (FarmActor :type "Actor Object Reference") (Amount :type "Float (double-precision)"))
  ;[1 0.02544 0.1955] SERVER EVENTS
  ;;[1 1 1] ADD WATER
  (`self.AddWater` FarmActor Amount))

(event `CL_SendFeedbackToClient`
  (params (Message :type Text))
  ;[0.2546 1 0.2921] CLIENT EVENTS
  ;;[1 1 1] SEND FEEDBACK TO CLIENT
  (`self.SendFeedbackToClient` Message))

(event `SRV_HarvestPlant`
  (params (FarmActor :type "Actor Object Reference"))
  ;[1 0.02544 0.1955] SERVER EVENTS
  ;;[1 1 1] HARVEST PLANT
  (bind _canharvest (`self.CheckCanHarvest` FarmActor))
  (if _canharvest
    ;;;[0 1 0.09849] INSERT LOGIC TO HANDLE REWARD WHEN HARVESTING
    (bind _plantdata (message `/Game/FarmingSystem/Blueprints/Interfaces/BPI_FarmingSystem.BPI_GetPlantData` FarmActor))
    (message `/Game/FarmingSystem/Blueprints/Interfaces/BPI_FarmingSystem.BPI_ResetFarmActor` FarmActor)))

(event `CL_RemovePlantSelectionWidget`
  ;[0.2546 1 0.2921] CLIENT EVENTS
  ;;[1 1 1] REMOVE PLANT SELECTION WIDGET
  (`self.RemovePlantSelectionWidget`))

(fn `AddWater`
  (params (Actor :type "Actor Object Reference") (Amount :type "Float (double-precision)"))
  (locals (LocalAmount :type "Float (double-precision)") (LocalActor :type "Actor Object Reference"))
  (set `local.LocalActor` Actor)
  (set `local.LocalAmount` Amount)
  (bind (_plantdata _plantstate) (message `/Game/FarmingSystem/Blueprints/Interfaces/BPI_FarmingSystem.BPI_GetPlantData` (`local.LocalActor`)))
  (if (< (`.CurrentWaterAmount_10_079907774EDF4B4A7342EB8053F626EA` (break `/Game/FarmingSystem/Blueprints/Data/Structs/STR_PlantState` _plantstate)) 100.0)
    (`self.ValidatePlayerDistance` (`local.LocalActor`)
      (:`InDistance`
        (message `/Game/FarmingSystem/Blueprints/Interfaces/BPI_FarmingSystem.BPI_AddWater` (`local.LocalActor`) (`local.LocalAmount`))
        (return))
      (:`OutOfDistance`
        (`self.CL_SendFeedbackToClient` "YOU'RE TOO FAR AWAY TO ADD WATER")))
    (else
      (`self.CL_SendFeedbackToClient` "NO WATER NEEDED")
      (return))))

(fn `CheckCanHarvest`
  (params (FarmActor :type "Actor Object Reference"))
  (returns (CanHarvest :type Boolean))
  (bind (_plantdata _plantstate) (message `/Game/FarmingSystem/Blueprints/Interfaces/BPI_FarmingSystem.BPI_GetPlantData` FarmActor))
  (if (`.FinishedGrowing_3_2F31DF0645566BA76D38C98D3ACAB7A4` (break `/Game/FarmingSystem/Blueprints/Data/Structs/STR_PlantState` _plantstate))
    (`self.ValidatePlayerDistance` FarmActor
      (:`InDistance`
        (return true))
      (:`OutOfDistance`
        (`self.CL_SendFeedbackToClient` "YOU'RE TOO FAR AWAY TO HARVEST")
        (return false)))
    (else
      (`self.CL_SendFeedbackToClient` "NOT READY TO HARVEST")
      (return false))))

(fn `CheckPlacementCollision`
  (returns (PlacementBlocked :type Boolean))
  (bind _farmactor (`self.FarmActor`))
  (bind _returnvalue (`Actor.K2_GetActorLocation` (`self.FarmActor`)))
  (`/Engine/EditorBlueprintResources/StandardMacros.IsValid` _farmactor
    (:`Is Valid`
      (bind _mesh (`/Game/FarmingSystem/Blueprints/BP_FarmActor.BPI_GetFarmActorMesh` _farmactor))
      (if (`self.bEnableCollisionCheck`)
        (bind (_returnvalue_origin _returnvalue_boxextent) (`KismetMathLibrary.BreakBoxSphereBounds` (`StaticMesh.GetBounds` (`StaticMeshComponent.StaticMesh` _mesh))))
        (bind _outhit (`KismetSystemLibrary.BoxTraceSingleForObjects` _returnvalue _returnvalue _returnvalue_boxextent (`SceneComponent.K2_GetComponentRotation` _mesh) (`|MakeArray` "ObjectTypeQuery2" :!type "EObjectTypeQuery Enum") false (`|MakeArray` (`self.FarmActor`) :!type "Actor Object Reference")))
        (cast `/Game/FarmingSystem/Blueprints/BP_FarmActor` (`.HitActor` (`GameplayStatics.BreakHitResult` _outhit))
          (:`then`
            (return true))
          (:`CastFailed`
            (return false)))
        (else
          (return false))))))

(fn `CreatePlantSelectionWidget`
  (params (FarmActor :type "Actor Object Reference"))
  (`/Engine/EditorBlueprintResources/StandardMacros.IsValid` (`self.PlantSelectionWidget`)
    (:`Is Valid`
      (`Widget.RemoveFromParent` (`self.PlantSelectionWidget`)))
    (:`Is Not Valid`
      _))
  (bind _returnvalue (`|CreateWidget` "/Game/FarmingSystem/Blueprints/Widgets/WBP_SelectPlant.WBP_SelectPlant_C" (`self.GetController`) FarmActor))
  (bind _output_get (set `self.PlantSelectionWidget` _returnvalue))
  (`UserWidget.AddToViewport` _output_get 0)
  (`WidgetBlueprintLibrary.SetInputMode_GameAndUIEx` (`self.GetController`) (`self.PlantSelectionWidget`))
  (set `PlayerController.bShowMouseCursor` true (`self.GetController`))
  (return))

(fn `FinalizePlacement`
  (if (`self.bPlacementState`)
    (bind _placementblocked (`self.CheckPlacementCollision`))
    (if _placementblocked
      (`self.CL_SendFeedbackToClient` "PLACEMENT IS BLOCKED")
      (else
        (`self.CL_SendFeedbackToClient` "PLACED FARM ACTOR")
        (`self.SRV_AddWater` (`self.FarmActor`) (`self.FarmActorDefaultWaterAmount`))
        (set `self.FarmActor` null)
        (`KismetSystemLibrary.K2_ClearAndInvalidateTimerHandle` (`self.UpdateFarmActorLocationTimer`))
        (set `self.bPlacementState` false)
        (return)))
    (else
      (return))))

(fn `FindCameraViewPoint`
  (returns (OutHit :type "HitResult Structure"))
  (locals (LocalTraceLocation :type "Vector Structure" :default (0.0 0.0 0.0)) (LocalTraceRotation :type "Rotator Structure" :default (struct)))
  (bind _localtracerotation (`local.LocalTraceRotation`))
  (bind _returnvalue (`KismetMathLibrary.GetForwardVector` _localtracerotation))
  (bind _playercameramanager (`PlayerController.PlayerCameraManager` (`self.GetController`)))
  (bind _returnvalue_2 (+ (* _returnvalue 10.0) (`local.LocalTraceLocation`)))
  (set `local.LocalTraceLocation` (`PlayerCameraManager.GetCameraLocation` _playercameramanager))
  (set `local.LocalTraceRotation` (`PlayerCameraManager.GetCameraRotation` _playercameramanager))
  (bind _outhit (`KismetSystemLibrary.BoxTraceSingle` _returnvalue_2 (+ _returnvalue_2 (* _returnvalue 1000.0)) (10.0 10.0 10.0) _localtracerotation "TraceTypeQuery1" false (`|MakeArray` (`self.OwningActor`) (`self.FarmActor`) :!type "Actor Object Reference")))
  (return _outhit))

(fn `FindClosestPlacementPoint`
  (params (GeneratedPoints :type "Array of Vector Structure") (Location :type "Vector Structure"))
  (returns (ClosestPoint :type "Vector Structure"))
  (locals (LocalArray :type "Array of Vector Structure") (LocalLocation :type "Vector Structure") (LocalCachedLength :type "Float (double-precision)" :default 0.0) (LocalCachedArrayIndex :type Integer :default 0) (LocalCachedVector :type "Vector Structure"))
  (set `local.LocalArray` GeneratedPoints)
  (set `local.LocalLocation` Location)
  (bind _output_get (set `local.LocalCachedVector` (`|GetArrayItem` (`local.LocalArray`))))
  (set `local.LocalCachedLength` (`KismetMathLibrary.VSize` (- _output_get (`local.LocalLocation`))))
  (for _array_element (`local.LocalArray`)
    (bind _returnvalue (`KismetMathLibrary.VSize` (- _array_element (`local.LocalLocation`))))
    (if (< _returnvalue (`local.LocalCachedLength`))
      (set `local.LocalCachedVector` _array_element)
      (set `local.LocalCachedLength` _returnvalue)))
  (return (`local.LocalCachedVector`)))

(fn `FindInteractableObjects`
  (set `/Game/FarmingSystem/Blueprints/Widgets/WBP_HUD.bCanInteract` (`KismetSystemLibrary.DoesImplementInterface` (`.HitActor` (`GameplayStatics.BreakHitResult` (`self.FindCameraViewPoint`))) "/Game/FarmingSystem/Blueprints/Interfaces/BPI_FarmingSystem.BPI_FarmingSystem_C") (`self.HUD`))
  (return))

(fn `GeneratePlacementPoints`
  (params (Actor :type "Actor Object Reference"))
  (returns (ClosestPoint :type "Vector Structure"))
  (locals (LocalFarmActorLocation :type "Vector Structure" :default (0.0 0.0 0.0)) (LocalRightVector :type "Vector Structure") (LocalForwardVector :type "Vector Structure" :default (0.0 0.0 0.0)) (LocalGeneratedPoints :type "Array of Vector Structure") (LocalMeshSize :type "Float (double-precision)") (LocalActor :type "Actor Object Reference"))
  (bind (_meshextent _scale) (`self.GetActorMeshExtent` (`local.LocalActor`)))
  (bind _returnvalue (`Actor.K2_GetActorRotation` (`local.LocalActor`)))
  (bind _returnvalue_2 (+ (.x _scale) (.y _scale)))
  (bind _returnvalue_3 (* (`local.LocalRightVector`) (+ (`local.LocalMeshSize`) (* (/ (.y (* _meshextent _scale)) 2.0) _returnvalue_2))))
  (bind _returnvalue_4 (* (`local.LocalForwardVector`) (+ (`local.LocalMeshSize`) (* (/ (.x (* _meshextent _scale)) 2.0) _returnvalue_2))))
  (set `local.LocalActor` Actor)
  (set `local.LocalFarmActorLocation` (`Actor.K2_GetActorLocation` (`local.LocalActor`)))
  (bind _mesh (message `/Game/FarmingSystem/Blueprints/Interfaces/BPI_FarmingSystem.BPI_GetFarmActorMesh` (`local.LocalActor`)))
  (bind (_returnvalue_origin _returnvalue_boxextent) (`KismetMathLibrary.BreakBoxSphereBounds` (`StaticMesh.GetBounds` (`StaticMeshComponent.StaticMesh` _mesh))))
  (set `local.LocalMeshSize` (+ (.x _returnvalue_boxextent) (.y _returnvalue_boxextent)))
  (set `local.LocalRightVector` (`KismetMathLibrary.GetRightVector` _returnvalue))
  (set `local.LocalForwardVector` (`KismetMathLibrary.GetForwardVector` _returnvalue))
  (`KismetArrayLibrary.Array_Add` (`local.LocalGeneratedPoints`) (+ (`local.LocalFarmActorLocation`) _returnvalue_4))
  (`KismetArrayLibrary.Array_Add` (`local.LocalGeneratedPoints`) (+ (`local.LocalFarmActorLocation`) (* _returnvalue_4 -1.0)))
  (`KismetArrayLibrary.Array_Add` (`local.LocalGeneratedPoints`) (+ (`local.LocalFarmActorLocation`) _returnvalue_3))
  (`KismetArrayLibrary.Array_Add` (`local.LocalGeneratedPoints`) (+ (`local.LocalFarmActorLocation`) (* _returnvalue_3 -1.0)))
  (return (`self.FindClosestPlacementPoint` (`local.LocalGeneratedPoints`) (`.Location` (`GameplayStatics.BreakHitResult` (`self.FindCameraViewPoint`))))))

(fn `GetActorMeshExtent`
  (params (Actor :type "Actor Object Reference"))
  (returns (MeshExtent :type "Vector Structure") (Scale :type "Vector Structure"))
  (bind _mesh (message `/Game/FarmingSystem/Blueprints/Interfaces/BPI_FarmingSystem.BPI_GetFarmActorMesh` Actor))
  (bind (_returnvalue_origin _returnvalue_boxextent) (`KismetMathLibrary.BreakBoxSphereBounds` (`StaticMesh.GetBounds` (`StaticMeshComponent.StaticMesh` _mesh))))
  (return _returnvalue_boxextent (`SceneComponent.K2_GetComponentScale` _mesh)))

(fn `GetController`
  (returns (`AsPlayer Controller` :type "PlayerController Object Reference"))
  (locals (LocalController :type "PlayerController Object Reference"))
  (bind _aspawn (cast `Pawn` (`self.OwningActor`))
    (:`then`
      (bind _asplayer_controller (cast `PlayerController` (`Pawn.GetController` _aspawn)))
      (set `local.LocalController` _asplayer_controller))
    (:`CastFailed`
      (bind _asplayer_controller_2 (cast `PlayerController` (`self.OwningActor`)))
      (set `local.LocalController` _asplayer_controller_2)))
  (return (`local.LocalController`)))

(fn `GetFarmActorPlacementLocation`
  (returns (ReturnValue :type "Vector Structure"))
  (locals (LocalHitActor :type "Actor Object Reference") (LocalHitLocation :type "Vector Structure"))
  (bind (_bblockinghit _binitialoverlap _time _distance _location _impactpoint _normal _impactnormal _physmat _hitactor) (`GameplayStatics.BreakHitResult` (`self.FindCameraViewPoint`)))
  (set `local.LocalHitLocation` _impactpoint)
  (set `local.LocalHitActor` _hitactor)
  (if (`self.bEnableSnapping`)
    (if (`KismetSystemLibrary.DoesImplementInterface` (`local.LocalHitActor`) "/Game/FarmingSystem/Blueprints/Interfaces/BPI_FarmingSystem.BPI_FarmingSystem_C")
      (return (`self.GeneratePlacementPoints` (`local.LocalHitActor`)))
      (else
        _)))
  (return (`local.LocalHitLocation`)))

(fn `GetSpawnTransform`
  (returns (ReturnValue :type "Transform Structure"))
  (bind _returnvalue (`Controller.K2_GetPawn` (`self.GetController`)))
  (return (`KismetMathLibrary.MakeTransform` (+ (`Actor.K2_GetActorLocation` _returnvalue) (* (`KismetMathLibrary.GetForwardVector` (`Actor.K2_GetActorRotation` _returnvalue)) 200.0)))))

(fn `OnRep_bPlacementBlocked`
  (`/Engine/EditorBlueprintResources/StandardMacros.IsValid` (`self.FarmActor`)
    (:`Is Valid`
      (`PrimitiveComponent.SetMaterial` (`/Game/FarmingSystem/Blueprints/BP_FarmActor.Soil` (`self.FarmActor`)) 0 (select `bool` (`self.bPlacementBlocked`) :`false` (`self.FarmActorDefaultMaterial`) :`true` "/Game/FarmingSystem/Materials/M_PlacementDisabled.M_PlacementDisabled")))))

(fn `OnRep_FarmActorTransform`
  (`Actor.K2_SetActorTransform` (`self.FarmActor`) (`self.FarmActorTransform`) false false)
  (return))

(fn `PlantSeed`
  (params (Actor :type "Actor Object Reference") (PlantData :type "/Game/FarmingSystem/Blueprints/Data/Structs/STR_FarmingSystem Structure"))
  (bind (_plantdata _plantstate) (message `/Game/FarmingSystem/Blueprints/Interfaces/BPI_FarmingSystem.BPI_GetPlantData` Actor))
  (if (`.SeedPlanted_1_15E3D9AB4465F80843FB5D9848F33BE6` (break `/Game/FarmingSystem/Blueprints/Data/Structs/STR_PlantState` _plantstate))
    (`self.CL_SendFeedbackToClient` "A SEED IS ALREADY PLANTED")
    (return)
    (else
      (message `/Game/FarmingSystem/Blueprints/Interfaces/BPI_FarmingSystem.BPI_SetPlantData` Actor PlantData)
      (if (`self.bClosePlantSelectionWhenPlanted`)
        (`self.CL_RemovePlantSelectionWidget`))
      (`self.CL_SendFeedbackToClient` "SEED PLANTED")
      (return))))

(fn `RemovePlantSelectionWidget`
  (bind _asplayer_controller (`self.GetController`))
  (`/Engine/EditorBlueprintResources/StandardMacros.IsValid` (`self.PlantSelectionWidget`)
    (:`Is Valid`
      (`Widget.RemoveFromParent` (`self.PlantSelectionWidget`)))
    (:`Is Not Valid`
      _))
  (`WidgetBlueprintLibrary.SetInputMode_GameOnly` _asplayer_controller)
  (set `PlayerController.bShowMouseCursor` false _asplayer_controller))

(fn `SendFeedbackToClient`
  (params (Message :type Text))
  (bind _messages (`/Game/FarmingSystem/Blueprints/Widgets/WBP_HUD.Messages` (`self.HUD`)))
  (`/Engine/EditorBlueprintResources/StandardMacros.IsValid` (`self.HUD`)
    (:`Is Valid`
      (bind _returnvalue (`|CreateWidget` "/Game/FarmingSystem/Blueprints/Widgets/WBP_Message.WBP_Message_C" (`self.GetController`) Message))
      (`PanelWidget.AddChild` _messages _returnvalue)
      (`ScrollBox.ScrollToEnd` _messages)
      (return))
    (:`Is Not Valid`
      (return))))

(fn `SetFarmingState`
  (params (bFarmingState :type Boolean))
  (bind _output_get (set `self.bPlacementState` bFarmingState))
  (if _output_get
    (`self.CL_SendFeedbackToClient` "PLACEMENT ENABLED")
    (`self.SRV_SpawnFarmActor`)
    (bind _returnvalue (`KismetSystemLibrary.K2_SetTimerDelegate` (`|CreateDelegate` :!event `CL_UpdateFarmActorPlacementLocation`) (`self.PlacementUpdateRate`) true))
    (set `self.UpdateFarmActorLocationTimer` _returnvalue)
    (return)
    (else
      (`self.CL_SendFeedbackToClient` "PLACEMENT DISABLED")
      (`/Engine/EditorBlueprintResources/StandardMacros.IsValid` (`self.FarmActor`)
        (:`Is Valid`
          (`Actor.K2_DestroyActor` (`self.FarmActor`))
          (set `self.FarmActor` null)
          (`KismetSystemLibrary.K2_ClearAndInvalidateTimerHandle` (`self.UpdateFarmActorLocationTimer`))
          (return))))))

(fn `SpawnFarmActor`
  (bind _asplayer_controller (`self.GetController`))
  (bind _returnvalue (`|SpawnActorFromClass` (`self.FarmActorToSpawn`) (`self.GetSpawnTransform`) "AlwaysSpawn" "OverrideRootScale" _asplayer_controller (`Controller.K2_GetPawn` _asplayer_controller)))
  (set `self.FarmActor` _returnvalue)
  (bind _mesh (`/Game/FarmingSystem/Blueprints/BP_FarmActor.BPI_GetFarmActorMesh` (`self.FarmActor`)))
  (set `self.FarmActorDefaultMaterial` (`|GetArrayItem` (`MeshComponent.GetMaterials` _mesh)))
  (return))

(fn `UpdateFarmActorPlacementLocation`
  (`/Engine/EditorBlueprintResources/StandardMacros.IsValid` (`self.FarmActor`)
    (:`Is Valid`
      (bind _placementblocked (`self.CheckPlacementCollision`))
      (set `self.bPlacementBlocked` _placementblocked)
      (bind _output_get (set `self.FarmActorTransform` (`KismetMathLibrary.MakeTransform` (`self.GetFarmActorPlacementLocation`) (`self.FarmActorRotation`))))
      (`self.SRV_UpdateFarmActorLocation` _output_get))
    (:`Is Not Valid`
      (return))))